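; Interactable med pack pickup for the ALS-based player character, shown as a glowing sphere until the player comes near.
; Entering the trigger sphere swaps the glow for a hologram with widgets and light, plays a cue, and registers it as the player's InteractObject; leaving clears that reference.
; Tick yaws the arrow toward the player.
; Interact increments the player's med pack count, plays a sound and destroys the actor.
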(event `self.ReceiveBeginPlay`
  ;[1 0.6723 0.4679] Set hologram effect to be hidden and set reference to player
  (`SceneComponent.SetHiddenInGame` (`self.Arrow`) true true)
  (`SceneComponent.SetHiddenInGame` (`self.SM_Print_Model`) true true)
  (bind _asals_anim_man_character_bp (cast `/Game/AdvancedLocomotionV4/Blueprints/CharacterLogic/ALS_AnimMan_CharacterBP` (`GameplayStatics.GetPlayerCharacter` 0)))
  (set `self.MyChar` _asals_anim_man_character_bp))

(event `self.ReceiveTick`
  (params (DeltaSeconds :type "Float (single-precision)"))
  (bind _arrow (`self.Arrow`))
  (bind (_returnvalue_roll _returnvalue_pitch) (`KismetMathLibrary.BreakRotator` (`SceneComponent.K2_GetComponentRotation` _arrow)))
  (bind (_returnvalue_roll_2 _returnvalue_pitch_2 _returnvalue_yaw) (`KismetMathLibrary.BreakRotator` (`KismetMathLibrary.FindLookAtRotation` (`SceneComponent.K2_GetComponentLocation` (`self.Arrow`)) (`self.K2_GetActorLocation` (`GameplayStatics.GetPlayerCharacter` 0)))))
  ;[1 0.7573 0.3395] Keep widgets facing the player
  (`SceneComponent.K2_SetWorldRotation` _arrow (`KismetMathLibrary.MakeRotator` _returnvalue_roll _returnvalue_pitch (- _returnvalue_yaw 25.0)) false false))

(event `self.Sphere1.OnComponentBeginOverlap`
  (params (OverlappedComponent :type "PrimitiveComponent Object Reference") (OtherActor :type "Actor Object Reference") (OtherComp :type "PrimitiveComponent Object Reference") (OtherBodyIndex :type Integer) (bFromSweep :type Boolean) (SweepResult :type "HitResult Structure (by ref)"))
  ;[1 0.7569 0.2249] When player enters the collision
  (bind _asals_anim_man_character_bp (cast `/Game/AdvancedLocomotionV4/Blueprints/CharacterLogic/ALS_AnimMan_CharacterBP` OtherActor))
  ;[1 0.6824 0.1812] Show  hologram effect, widgets and light
  (`SceneComponent.SetHiddenInGame` (`self.SM_Print_Model`) false true)
  (`SceneComponent.SetHiddenInGame` (`self.RectLight`) false true)
  (`SceneComponent.SetHiddenInGame` (`self.Widget`) false true)
  (`SceneComponent.SetHiddenInGame` (`self.Widget1`) false true)
  (set `/Game/AdvancedLocomotionV4/Blueprints/CharacterLogic/ALS_AnimMan_CharacterBP.InteractObject` self _asals_anim_man_character_bp)
  (`SceneComponent.SetHiddenInGame` (`self.Sphere`) true true)
  (`/Engine/EditorBlueprintResources/StandardMacros.DoOnce` false :!label _label
    (:`Completed`
      (`ActorComponent.Activate` (`self.Health_Pickup_5_Cue`) true))))

(event `self.Sphere1.OnComponentEndOverlap`
  (params (OverlappedComponent :type "PrimitiveComponent Object Reference") (OtherActor :type "Actor Object Reference") (OtherComp :type "PrimitiveComponent Object Reference") (OtherBodyIndex :type Integer))
  ;[1 0.7117 0.185] When player exits the collision
  (bind _asals_anim_man_character_bp (cast `/Game/AdvancedLocomotionV4/Blueprints/CharacterLogic/ALS_AnimMan_CharacterBP` OtherActor))
  ;[1 0.7679 0.4393] Hide hologram effect and show sphere glowing object
  (`SceneComponent.SetHiddenInGame` (`self.Arrow`) true true)
  (`SceneComponent.SetHiddenInGame` (`self.SM_Print_Model`) true true)
  (set `/Game/AdvancedLocomotionV4/Blueprints/CharacterLogic/ALS_AnimMan_CharacterBP.InteractObject` null _asals_anim_man_character_bp)
  (`SceneComponent.SetHiddenInGame` (`self.Sphere`) false true)
  (goto _label :!via `Reset`))

(event `self.Interact`
  ;[1 0.6083 0.1131] On activation add the inventory item
  (`/Engine/EditorBlueprintResources/StandardMacros.IncrementInt` (`/Game/AdvancedLocomotionV4/Blueprints/CharacterLogic/ALS_AnimMan_CharacterBP.MedPackAmt` (`self.MyChar`))
    (:`  `
      (`self.K2_DestroyActor`)
      (`GameplayStatics.PlaySoundAtLocation` "/Game/Audio/Ultimate_SFX_Bundle/Sci_Fi_Weapon_Sounds/Wavs/Weapon_Swap/Weapon_Swap_4.Weapon_Swap_4" (`self.K2_GetActorLocation`) (struct) 1.0 1.0 0.0 null null null)
      (`self.K2_DestroyActor`))))

(fn `UserConstructionScript`)