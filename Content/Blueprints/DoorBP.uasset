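; Interactive sliding door that opens when the player activates it and closes automatically once the player moves away.
; The collision box registers the door as the ALS character's InteractObject and drives two prompt widgets' highlight states.
; Interact plays widget animation and sound, then a timeline slides the door mesh along clamped local Y, reversed for closing.
; Tick checks player distance to trigger closing, and the construction script tints the door through a dynamic material.
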(event `self.ReceiveBeginPlay`
  ;[1 0.7627 0.3896] Set Door Widget References
  (set `self.DoorWidget1` (cast `/Game/Blueprints/UI/DoorUI/DoorWidget` (`WidgetComponent.GetUserWidgetObject` (`self.Widget`)) :!pure true))
  (set `self.DoorWidget2` (cast `/Game/Blueprints/UI/DoorUI/DoorWidget` (`WidgetComponent.GetUserWidgetObject` (`self.Widget1`)) :!pure true)))

(event `Open`
  (bind (_relativelocation_x _relativelocation_y _relativelocation_z) (`KismetMathLibrary.BreakVector` (`SceneComponent.RelativeLocation` (`self.SM_Door_A_part`))))
  (bind (_relativelocation_x_2 _relativelocation_y_2) (`KismetMathLibrary.BreakVector` (`SceneComponent.RelativeLocation` (`self.SM_Door_A_part`))))
  ;[1 0.6144 0.1961] Door Movement
  (`SceneComponent.SetHiddenInGame` (`self.Widget`) true false)
  (`SceneComponent.SetHiddenInGame` (`self.Widget1`) true false)
  (set `self.Direction` 1.0)
  (set `self.RelativeLocationY` _relativelocation_y_2)
  (bind (_direction _doorlocy) (`Timeline|OpenDoor` :!via `PlayFromStart` :!label _label)
    (:`Update`
      (set `self.RelativeLocationY` (`KismetMathLibrary.FClamp` (+ (`self.RelativeLocationY`) (* _doorlocy (`self.Direction`))) 0.0 160.0))
      (`SceneComponent.K2_SetRelativeLocation` (`self.SM_Door_A_part`) (`KismetMathLibrary.MakeVector` _relativelocation_x (`self.RelativeLocationY`) _relativelocation_z) false false))
    (:`Finished`
      (set `self.DoorOpen` (== (`self.Direction`) 1.0))
      (if (not (`self.DoorOpen`))
        (`/Game/Blueprints/UI/DoorUI/DoorWidget.SetFlashing` (`self.DoorWidget1`) true)
        (`/Game/Blueprints/UI/DoorUI/DoorWidget.SetFlashing` (`self.DoorWidget2`) true)
        (`SceneComponent.SetHiddenInGame` (`self.Widget`) false false)
        (`SceneComponent.SetHiddenInGame` (`self.Widget1`) false false)))))

(event `Close`
  (bind (_relativelocation_x _relativelocation_y) (`KismetMathLibrary.BreakVector` (`SceneComponent.RelativeLocation` (`self.SM_Door_A_part`))))
  ;[1 0.6144 0.1961] Door Movement
  (`self.SetDoorSound` false)
  (`KismetSystemLibrary.Delay` 1.0)
  (set `self.Direction` -0.5)
  (set `self.RelativeLocationY` _relativelocation_y)
  (goto _label :!via `ReverseFromEnd`))

(event `self.ReceiveTick`
  (params (DeltaSeconds :type "Float (single-precision)"))
  ;[1 0.4777 0.1506] Close the door if player is not close to it
  (if (`self.DoorOpen`)
    (bind _distance (`self.GetDistanceToPlayer` :!label _label_2))
    (if (> _distance 200.0)
      (`/Engine/EditorBlueprintResources/StandardMacros.DoOnce` false :!label _label_3
        (:`Completed`
          (`self.Close`)
          (`KismetSystemLibrary.Delay` 4.0)
          (`|ExecutionSequence`
            (:`then_0`
              (goto _label_2))
            (:`then_1`
              (goto _label_3 :!via `Reset`))))))))

(event `CheckDoorOpen`
  ;[1 0.4777 0.1506] Close the door if player is not close to it
  (goto _label_2))

(event `self.Interact`
  ;[1 0.6969 0.2395] On Activation
  (if (not (`self.DoorOpen`))
    (`/Game/Blueprints/UI/DoorUI/DoorWidget.RotateCircles` (`self.DoorWidget1`))
    (`/Game/Blueprints/UI/DoorUI/DoorWidget.RotateCircles` (`self.DoorWidget2`))
    (`self.SetDoorSound` true)
    (`KismetSystemLibrary.Delay` 1.5)
    (`self.Open`)))

(event `self.Box.OnComponentBeginOverlap`
  (params (OverlappedComponent :type "PrimitiveComponent Object Reference") (OtherActor :type "Actor Object Reference") (OtherComp :type "PrimitiveComponent Object Reference") (OtherBodyIndex :type Integer) (bFromSweep :type Boolean) (SweepResult :type "HitResult Structure (by ref)"))
  ;[1 0.6626 0.2746] When entering into the collision box of the door
  (bind _asals_anim_man_character_bp (cast `/Game/AdvancedLocomotionV4/Blueprints/CharacterLogic/ALS_AnimMan_CharacterBP` OtherActor))
  (`|ExecutionSequence`
    (:`then_0`
      (goto _label_5 :!via `Reset`))
    (:`then_1`
      (`/Engine/EditorBlueprintResources/StandardMacros.DoOnce` false :!label _label_4
        (:`Completed`
          (set `/Game/AdvancedLocomotionV4/Blueprints/CharacterLogic/ALS_AnimMan_CharacterBP.InteractObject` self _asals_anim_man_character_bp)
          (`/Game/Blueprints/UI/DoorUI/DoorWidget.SetFlashing` (`self.DoorWidget1`) false)
          (`/Game/Blueprints/UI/DoorUI/DoorWidget.SetFlashing` (`self.DoorWidget2`) false)
          (`/Game/Blueprints/UI/DoorUI/DoorWidget.Brighten` (`self.DoorWidget1`))
          (`/Game/Blueprints/UI/DoorUI/DoorWidget.Brighten` (`self.DoorWidget2`)))))))

(event `self.Box.OnComponentEndOverlap`
  (params (OverlappedComponent :type "PrimitiveComponent Object Reference") (OtherActor :type "Actor Object Reference") (OtherComp :type "PrimitiveComponent Object Reference") (OtherBodyIndex :type Integer))
  ;[1 0.6626 0.2746] When entering into the collision box of the door
  (bind _asals_anim_man_character_bp (cast `/Game/AdvancedLocomotionV4/Blueprints/CharacterLogic/ALS_AnimMan_CharacterBP` OtherActor))
  (`|ExecutionSequence`
    (:`then_0`
      (goto _label_4 :!via `Reset`))
    (:`then_1`
      (`/Engine/EditorBlueprintResources/StandardMacros.DoOnce` false :!label _label_5
        (:`Completed`
          (`/Game/Blueprints/UI/DoorUI/DoorWidget.Darken` (`self.DoorWidget1`))
          (`/Game/Blueprints/UI/DoorUI/DoorWidget.Darken` (`self.DoorWidget2`))
          (set `/Game/AdvancedLocomotionV4/Blueprints/CharacterLogic/ALS_AnimMan_CharacterBP.InteractObject` null _asals_anim_man_character_bp)
          (`/Game/Blueprints/UI/DoorUI/DoorWidget.Darken` (`self.DoorWidget1`))
          (`/Game/Blueprints/UI/DoorUI/DoorWidget.Darken` (`self.DoorWidget2`))
          (`self.CheckDoorOpen`))))))

(fn `GetDistanceToPlayer`
  (returns (Distance :type "Float (double-precision)"))
  (return (`self.GetDistanceTo` (`GameplayStatics.GetPlayerCharacter` 0) self)))

(fn `SetDoorSound`
  (params (IsOpening :type Boolean))
  (bind _door_open_9_cue (`self.DOOR_OPEN_9_Cue`))
  (if IsOpening
    (`AudioComponent.SetSound` _door_open_9_cue "/Game/Audio/Ultimate_SFX_Bundle/Sci-Fi_Doors_Pro/Cues/Doors_Opening/DOOR_OPEN_35_Cue.DOOR_OPEN_35_Cue")
    (else
      (`AudioComponent.SetSound` _door_open_9_cue "/Game/Audio/Ultimate_SFX_Bundle/Sci-Fi_Doors_Pro/Cues/Doors_Closing/DOOR_CLOSE_19_Cue.DOOR_CLOSE_19_Cue")))
  (`ActorComponent.Activate` _door_open_9_cue true))

(fn `UserConstructionScript`
  (bind _returnvalue (`PrimitiveComponent.CreateDynamicMaterialInstance` (`self.SM_Door_A_part`) 1 "/Game/SciFiModularEnvironment/Materials/MI_Painted_Metal_Orange.MI_Painted_Metal_Orange" "None"))
  (`MaterialInstanceDynamic.SetVectorParameterValue` _returnvalue "Color" (`self.Value`)))