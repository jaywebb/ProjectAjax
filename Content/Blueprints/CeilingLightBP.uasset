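; Ceiling light Blueprint that switches its spotlight on or off based on how close the player is.
; From BeginPlay, an endless delay loop with a randomized interval of a few seconds calls CheckDistanceToPlayer instead of using Tick.
; That function measures the distance to the first player character and sets the spotlight to full intensity within range, or zero beyond it.
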(event `self.ReceiveBeginPlay`
  (`KismetSystemLibrary.Delay` (`KismetMathLibrary.RandomFloatInRange` 2.0 4.0) :!label _label)
  (`self.CheckDistanceToPlayer`)
  (goto _label))

(fn `CheckDistanceToPlayer`
  (bind _spotlight (`self.SpotLight`))
  (if (< (`self.GetDistanceTo` (`GameplayStatics.GetPlayerCharacter` 0) self) 2000.0)
    (`LightComponent.SetIntensity` _spotlight 8000.0)
    (else
      (`LightComponent.SetIntensity` _spotlight 0.0))))

(fn `UserConstructionScript`)