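; Player UI actor that presents objective, details and inventory text through widget components, alongside a main widget, panels and backgrounds.
; BeginPlay caches the typed widget references, sets the section titles and fills in the hard-coded opening mission objective and Ajax backstory.
; Helper functions toggle visibility per element group, set widget text, and play opening or closing sounds by swapping cues on two audio components.
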(event `self.ReceiveBeginPlay`
  (`|ExecutionSequence`
    (:`then_0`
      (set `self.ObjectiveUIWidget` (cast `/Game/Blueprints/UI/PlayerUI/PlayerUIText` (`WidgetComponent.GetUserWidgetObject` (`self.ObjectiveUI`)) :!pure true))
      (set `self.DetailsUIWidget` (cast `/Game/Blueprints/UI/PlayerUI/PlayerUIText` (`WidgetComponent.GetUserWidgetObject` (`self.DetailsUI`)) :!pure true))
      (set `self.InventoryUIWidget` (cast `/Game/Blueprints/UI/PlayerUI/InventoryUIText` (`WidgetComponent.GetUserWidgetObject` (`self.InventoryUI`)) :!pure true))
      (set `self.MainWidgetUI` (cast `/Game/Blueprints/UI/PlayerUI/PlayerWidget` (`WidgetComponent.GetUserWidgetObject` (`self.MainWidget`)) :!pure true)))
    (:`then_1`
      (`TextBlock.SetText` (`/Game/Blueprints/UI/PlayerUI/PlayerUIText.TextTitle` (`self.ObjectiveUIWidget`)) "OBJECTIVE: ")
      (`TextBlock.SetText` (`/Game/Blueprints/UI/PlayerUI/PlayerUIText.TextTitle` (`self.DetailsUIWidget`)) "DETAILS: ")
      (`TextBlock.SetText` (`/Game/Blueprints/UI/PlayerUI/InventoryUIText.TextTitle` (`self.InventoryUIWidget`)) "INVENTORY: "))
    (:`then_2`
      (`self.SetUIText` (`/Game/Blueprints/UI/PlayerUI/PlayerUIText.Description` (`self.ObjectiveUIWidget`)) "Get to the Medical Deck and find Marcus.")
      (`self.SetUIText` (`/Game/Blueprints/UI/PlayerUI/PlayerUIText.Description` (`self.DetailsUIWidget`)) "You were checking out a meteorite that hit the hull of the Ajax and found some strange alien artifact.  \n \nGunfire ripped open the hull, giving you a way back inside the Ajax.  Many screams of terror are heard from inside.  \n \nMarcus Holloway, a biologist,  \nis trapped in a research lab on the Medical deck and needs your help. "))))

(fn `HideElements`
  (params (MainWidget :type Boolean) (WidgetBackground :type Boolean) (WidgetPanels :type Boolean) (TextUI :type Boolean))
  (`SceneComponent.SetHiddenInGame` (`self.MainWidget`) MainWidget false)
  (`SceneComponent.SetHiddenInGame` (`self.WidgetBgd`) WidgetBackground false)
  (`SceneComponent.SetHiddenInGame` (`self.WidgetReverseSide`) WidgetBackground false)
  (`SceneComponent.SetHiddenInGame` (`self.WidgetPanels`) WidgetPanels false)
  (`SceneComponent.SetHiddenInGame` (`self.InventoryUI`) TextUI false)
  (`SceneComponent.SetHiddenInGame` (`self.ObjectiveUI`) TextUI false)
  (`SceneComponent.SetHiddenInGame` (`self.DetailsUI`) TextUI false))

(fn `PlayUISound`
  (params (IsOpening :type Boolean))
  (bind _unlocked_3_cue (`self.Unlocked_3_Cue`))
  (bind _unlocked_3_cue1 (`self.Unlocked_3_Cue1`))
  (if IsOpening
    (`AudioComponent.SetSound` _unlocked_3_cue "/Game/Audio/Ultimate_SFX_Bundle/Modern_Ui_Sounds/Cues/Unlocked/Unlocked_4_Cue1.Unlocked_4_Cue1")
    (`ActorComponent.Activate` _unlocked_3_cue true)
    (`AudioComponent.SetSound` _unlocked_3_cue1 "/Game/Audio/Ultimate_SFX_Bundle/Modern_Ui_Sounds/Cues/Drone_Sounds/Drone_sounds_17_Cue.Drone_sounds_17_Cue")
    (`ActorComponent.Activate` _unlocked_3_cue1 true)
    (else
      (`AudioComponent.SetSound` _unlocked_3_cue "/Game/Audio/Ultimate_SFX_Bundle/Modern_Ui_Sounds/Cues/Success/Success_7_Cue.Success_7_Cue")
      (`ActorComponent.Activate` _unlocked_3_cue true))))

(fn `SetUIText`
  (params (TextWidget :type "TextBlock Object Reference") (Text :type Text))
  (`TextBlock.SetText` TextWidget Text))

(fn `UserConstructionScript`)