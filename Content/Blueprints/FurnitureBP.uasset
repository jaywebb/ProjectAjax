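; Configurable furniture prop Blueprint that switches between table and computer variants, with an optional chair.
; The Construction Script reads HasComputer to pick the SM_Computer03 or SM_Computer06 mesh, and IsTable to show either the table or that computer mesh.
; HasChair assigns the chair mesh, with no branch to clear it when false.
; The Event Graph holds only disabled default events, so there is no runtime logic.
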(fn `UserConstructionScript`
  (`|ExecutionSequence`
    (:`then_0`
      (if (`self.HasComputer`)
        (`StaticMeshComponent.SetStaticMesh` (`self.SM_Computer06`) "/Game/SciFi_Medical_Room/Meshes/SM_Computer03.SM_Computer03")
        (else
          (`StaticMeshComponent.SetStaticMesh` (`self.SM_Computer06`) "/Game/SciFi_Medical_Room/Meshes/SM_Computer06.SM_Computer06"))))
    (:`then_1`
      (if (`self.IsTable`)
        (`SceneComponent.SetVisibility` (`self.SM_Table01`) true false)
        (`SceneComponent.SetVisibility` (`self.SM_Computer06`) false false)
        (else
          (`SceneComponent.SetVisibility` (`self.SM_Computer06`) true false)
          (`SceneComponent.SetVisibility` (`self.SM_Table01`) false false))))
    (:`then_2`
      (if (`self.HasChair`)
        (`StaticMeshComponent.SetStaticMesh` (`self.SM_Chair`) "/Game/SciFi_Medical_Room/Meshes/SM_Chair.SM_Chair")))))