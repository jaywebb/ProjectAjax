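; ProjectileBP is a projectile Blueprint that shows an impact effect and destroys itself when its Box component hits something.
; On hit it prints the struck bone name if there is one, then spawns a small hit particle at the HitLocation component's position before destruction.
; The construction script tints the PElectroLaser1 particle by converting a variable into its color-over-life vector parameter.
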(event `self.Box.OnComponentHit`
  (params (HitComponent :type "PrimitiveComponent Object Reference") (OtherActor :type "Actor Object Reference") (OtherComp :type "PrimitiveComponent Object Reference") (NormalImpulse :type "Vector Structure") (Hit :type "HitResult Structure (by ref)"))
  (if (not (== Hit_HitBoneName "None"))
    (`KismetSystemLibrary.PrintString` (`KismetStringLibrary.Conv_NameToString` Hit_HitBoneName)))
  (`GameplayStatics.SpawnEmitterAtLocation` "/Game/FXVarietyPack/Particles/P_ky_hit1.P_ky_hit1" (`SceneComponent.K2_GetComponentLocation` (`self.HitLocation`)) (struct) (0.25 0.25 0.25))
  (`self.K2_DestroyActor`))

(fn `UserConstructionScript`
  (`ParticleSystemComponent.SetVectorParameter` (`self.P_ElectroLaser1`) "InstanceColorScaleOverLife" (`KismetMathLibrary.Conv_LinearColorToVector` (`self.NewVar_0`))))