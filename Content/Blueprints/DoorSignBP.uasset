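; DoorSignBP is a door sign Blueprint that displays text through a DoorSignUI widget hosted in its Widget component.
; On BeginPlay it checks the cached widget reference and, while invalid, retries the cast via SetSignText after one-second delays.
; Once valid, it passes its text color, sign text and alternate text to the widget, then calls ScrollingText with its scrolling flag.
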(event `SetSignText`
  (set `self.As Door Sign UI` (cast `/Game/Blueprints/UI/DoorUI/DoorSignUI` (`WidgetComponent.GetUserWidgetObject` (`self.Widget`)) :!pure true)))

(event `self.ReceiveBeginPlay`
  (`/Engine/EditorBlueprintResources/StandardMacros.IsValid` (`self.As Door Sign UI`) :!label _label
    (:`Is Valid`
      (`TextBlock.SetColorAndOpacity` (`/Game/Blueprints/UI/DoorUI/DoorSignUI.Text` (`self.As Door Sign UI`)) (`self.In Color and Opacity`))
      (set `/Game/Blueprints/UI/DoorUI/DoorSignUI.SignText` (`self.SignText`) (`self.As Door Sign UI`))
      (set `/Game/Blueprints/UI/DoorUI/DoorSignUI.AlternateText` (`self.AlternateText`) (`self.As Door Sign UI`))
      (`/Game/Blueprints/UI/DoorUI/DoorSignUI.ScrollingText` (`self.As Door Sign UI`) (`self.IsScrollingText`)))
    (:`Is Not Valid`
      (`KismetSystemLibrary.Delay` 1.0)
      (`self.SetSignText`)
      (goto _label))))

(fn `UserConstructionScript`)