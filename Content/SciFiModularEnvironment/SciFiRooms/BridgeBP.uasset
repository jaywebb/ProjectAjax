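; BridgeBP is a modular sci-fi bridge room actor whose walls are configured through door toggles.
; Its construction script runs SetWallTypes before the parent's, switching back, front and right child actor components between two wall classes per boolean.
; Front walls reuse the back wall classes, and the back door flags drive opposite-named components (DoorBackRight sets WallBackLeft).
; The event graph holds no active logic.
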(fn `SetWallTypes`
  (bind _wallbackleft (`self.WallBackLeft`))
  (bind _wallbackright (`self.WallBackRight`))
  (bind _wallfrontleft (`self.WallFrontLeft`))
  (bind _wallright2 (`self.WallRight2`))
  (bind _wallfrontright (`self.WallFrontRight`))
  (bind _wallright1 (`self.WallRight1`))
  (`|ExecutionSequence`
    (:`then_0`
      (if (`self.DoorBackRight`)
        (`ChildActorComponent.SetChildActorClass` _wallbackleft "/Game/SciFiModularEnvironment/SciFiRooms/WallSMBack1.WallSMBack1_C")
        (else
          (`ChildActorComponent.SetChildActorClass` _wallbackleft "/Game/SciFiModularEnvironment/SciFiRooms/WallSMBack2.WallSMBack2_C"))))
    (:`then_1`
      (if (`self.DoorBackLeft`)
        (`ChildActorComponent.SetChildActorClass` _wallbackright "/Game/SciFiModularEnvironment/SciFiRooms/WallSMBack1.WallSMBack1_C")
        (else
          (`ChildActorComponent.SetChildActorClass` _wallbackright "/Game/SciFiModularEnvironment/SciFiRooms/WallSMBack2.WallSMBack2_C"))))
    (:`then_2`
      (if (`self.DoorFrontLeft`)
        (`ChildActorComponent.SetChildActorClass` _wallfrontleft "/Game/SciFiModularEnvironment/SciFiRooms/WallSMBack1.WallSMBack1_C")
        (else
          (`ChildActorComponent.SetChildActorClass` _wallfrontleft "/Game/SciFiModularEnvironment/SciFiRooms/WallSMBack2.WallSMBack2_C"))))
    (:`then_3`
      (if (`self.DoorFrontRight`)
        (`ChildActorComponent.SetChildActorClass` _wallfrontright "/Game/SciFiModularEnvironment/SciFiRooms/WallSMBack1.WallSMBack1_C")
        (else
          (`ChildActorComponent.SetChildActorClass` _wallfrontright "/Game/SciFiModularEnvironment/SciFiRooms/WallSMBack2.WallSMBack2_C"))))
    (:`then_4`
      (if (`self.DoorRight1`)
        (`ChildActorComponent.SetChildActorClass` _wallright1 "/Game/SciFiModularEnvironment/SciFiRooms/WallSMRight1.WallSMRight1_C")
        (else
          (`ChildActorComponent.SetChildActorClass` _wallright1 "/Game/SciFiModularEnvironment/SciFiRooms/WallSMRight2.WallSMRight2_C"))))
    (:`then_5`
      (if (`self.DoorRight2`)
        (`ChildActorComponent.SetChildActorClass` _wallright2 "/Game/SciFiModularEnvironment/SciFiRooms/WallSMRight1.WallSMRight1_C")
        (else
          (`ChildActorComponent.SetChildActorClass` _wallright2 "/Game/SciFiModularEnvironment/SciFiRooms/WallSMRight2.WallSMRight2_C"))))))

(fn `UserConstructionScript`
  (`self.SetWallTypes`)
  (`parent.UserConstructionScript`))