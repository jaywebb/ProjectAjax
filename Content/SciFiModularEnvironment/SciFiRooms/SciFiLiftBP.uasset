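; Sci-fi lift Blueprint that drives a child LiftBox car toward a floor marker when interacted with.
; BeginPlay links itself to the LiftBox, targets the floor 1 marker, initializes the UI arrows and finds the LevelManager.
; Interact swaps visible levels for the current floor, then after a short delay sets the car's direction, speed and UI animations.
; The construction script applies a shared wall color to child wall actors.
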(event `self.ReceiveBeginPlay`
  (bind _movingup (`self.MovingUp`))
  (bind _liftui (`/Game/SciFiModularEnvironment/SciFiRooms/LiftBoxBP.LiftUI` (`self.LiftBoxRef`)))
  ;[1 0.5036 0.1971] When you begin play, create a reference to the LiftBox and the SciFiLiftBP . Set the first destination
  (bind _aslift_box_bp (cast `/Game/SciFiModularEnvironment/SciFiRooms/LiftBoxBP` (`ChildActorComponent.ChildActor` (`self.LiftBox`))))
  (bind _output_get (set `self.LiftBoxRef` _aslift_box_bp))
  (set `/Game/SciFiModularEnvironment/SciFiRooms/LiftBoxBP.SciFiLiftBP` self _output_get)
  (set `self.Destination` (`SceneComponent.K2_GetComponentLocation` (`self.Floor1Marker`)))
  ;[1 0.5739 0.1795] Rotate the Lift UI to the next  Destination
  (`/Game/Blueprints/UI/LIftUI/LIftWidget.SetDirection` (`/Game/Blueprints/LIftUIObject.LiftWidget` _liftui) _movingup)
  (`/Game/Blueprints/UI/LIftUI/LIftWidgetBgd.SetDirection` (`/Game/Blueprints/LIftUIObject.LiftWidgetBgd` _liftui) _movingup)
  ;[1 0.6059 0.2209] Set a reference to the Level Manager
  (bind _outactors (`GameplayStatics.GetAllActorsOfClass` "/Game/Blueprints/LevelManagerBP.LevelManagerBP_C"))
  (set `self.LevelManager` (`|GetArrayItem` _outactors)))

(event `self.Interact`
  (bind _liftboxref (`self.LiftBoxRef`))
  (bind (_destination_x _destination_y _destination_z) (`KismetMathLibrary.BreakVector` (`self.Destination`)))
  (bind (_liftcurrentloc_x _liftcurrentloc_y _liftcurrentloc_z) (`KismetMathLibrary.BreakVector` (`self.LiftCurrentLoc`)))
  (bind _liftboxref_2 (`self.LiftBoxRef`))
  (bind _liftboxref_3 (`self.LiftBoxRef`))
  (bind (_destination_x_2 _destination_y_2 _destination_z_2) (`KismetMathLibrary.BreakVector` (`self.Destination`)))
  (bind (_liftcurrentloc_x_2 _liftcurrentloc_y_2 _liftcurrentloc_z_2) (`KismetMathLibrary.BreakVector` (`self.LiftCurrentLoc`)))
  (bind _liftui (`/Game/SciFiModularEnvironment/SciFiRooms/LiftBoxBP.LiftUI` (`self.LiftBoxRef`)))
  (bind _liftwidget (`/Game/Blueprints/LIftUIObject.LiftWidget` _liftui))
  ;[1 0.6069 0.07832] If the lift is not moving
  (if (not (`/Game/SciFiModularEnvironment/SciFiRooms/LiftBoxBP.IsMoving` _liftboxref_2))
    (`/Game/SciFiModularEnvironment/SciFiRooms/LiftBoxBP.ResetFloorChange` _liftboxref_2)
    (if (== (`self.CurrentFloor`) 1)
      ;[1 0.4803 0.1953] Set the levels to be Hidden or Visible
      (`/Game/Blueprints/LevelManagerBP.UpdateVisibleLevels` (`self.LevelManager`) (`self.StartingFloorHIdeLevel`) (`self.StartingFloorShowLevel`))
      (else
        (`/Game/Blueprints/LevelManagerBP.UpdateVisibleLevels` (`self.LevelManager`) (`self.EndingFloorHideLevel`) (`self.EndingFloorShowLevel`))))
    (`KismetSystemLibrary.Delay` 1.0)
    ;[1 0.6811 0.3798] Check if you already at the destination. If so, show a message "You are at the destination"
    (set `self.LiftCurrentLoc` (`SceneComponent.K2_GetComponentLocation` (`/Game/SciFiModularEnvironment/SciFiRooms/LiftBoxBP.Door` (`self.LiftBoxRef`))))
    (if (`KismetMathLibrary.NearlyEqual_FloatFloat` _destination_z _liftcurrentloc_z)
      (`KismetSystemLibrary.PrintString` "Currently at the destination")
      (else
        ;[1 0.6784 0.3989] Check if the destination is above or below you. Set the Direction.
        (if (> _destination_z_2 _liftcurrentloc_z_2)
          (set `/Game/SciFiModularEnvironment/SciFiRooms/LiftBoxBP.Direction` 1.0 _liftboxref_3)
          (else
            (set `/Game/SciFiModularEnvironment/SciFiRooms/LiftBoxBP.Direction` -1.0 _liftboxref_3)))
        ;[1 0.8927 0.2891] Set the speed of lift movement
        (set `/Game/SciFiModularEnvironment/SciFiRooms/LiftBoxBP.Speed` (* (`self.BaseSpeed`) (`/Game/SciFiModularEnvironment/SciFiRooms/LiftBoxBP.Direction` _liftboxref)) _liftboxref)
        ;[1 0.4607 0.2487] Stop the Flashing Animation and Play the Moving Animation on the UI
        (`/Game/Blueprints/UI/LIftUI/LIftWidget.ShowFlashAnimation` _liftwidget false)
        (`/Game/Blueprints/UI/LIftUI/LIftWidgetBgd.ShowFlashAnimation` (`/Game/Blueprints/LIftUIObject.LiftWidgetBgd` _liftui) false)
        (`/Game/Blueprints/UI/LIftUI/LIftWidget.SetMoving` _liftwidget true)))))

(fn `UserConstructionScript`
  (for _array_element (`SceneComponent.GetChildrenComponents` (`self.DefaultSceneRoot`) false)
    (bind _aswall_base_bp (cast `/Game/SciFiModularEnvironment/SciFiRooms/WallBaseBP` (`ChildActorComponent.ChildActor` (cast `ChildActorComponent` _array_element :!pure true))))
    (`/Game/SciFiModularEnvironment/SciFiRooms/WallBaseBP.SetWallColor` _aswall_base_bp (`self.Wall Color`))))