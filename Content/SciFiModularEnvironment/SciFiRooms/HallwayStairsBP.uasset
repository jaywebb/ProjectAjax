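; Modular hallway staircase Blueprint that procedurally builds a run of stair sections from a section count.
; On construction it calls BuildStairs, then the parent construction script.
; BuildStairs adds one fewer HallwayStairSectionBP child actors than the count, placing the first at its own Arrow and chaining later ones from previous sections' Arrows.
; The final section has its stairs hidden; the event graph is unused.
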(fn `BuildStairs`
  (bind _returnvalue (- (`self.NumberOfSections`) 2))
  (set `self.ActorTransform` (`SceneComponent.K2_GetComponentToWorld` (`self.Arrow`)))
  (if (> (`self.NumberOfSections`) 1)
    (for _index (range (+ _returnvalue 1))
      (if (== _index _returnvalue)
        (bind _returnvalue_2 (`AddComponent|NODE_AddChildActorComponent-1` :`bManualAttachment` true :`RelativeTransform` (`self.ActorTransform`)))
        (`ChildActorComponent.SetChildActorClass` _returnvalue_2 "/Game/SciFiModularEnvironment/SciFiRooms/HallwayStairSectionBP.HallwayStairSectionBP_C")
        (bind _ashallway_stair_section_bp (cast `/Game/SciFiModularEnvironment/SciFiRooms/HallwayStairSectionBP` (`ChildActorComponent.ChildActor` _returnvalue_2)))
        (`KismetArrayLibrary.Array_AddUnique` (`self.StairSections`) _ashallway_stair_section_bp)
        (set `self.ActorTransform` (`SceneComponent.K2_GetComponentToWorld` (`/Game/SciFiModularEnvironment/SciFiRooms/HallwayStairSectionBP.Arrow` (`|GetArrayItem` (`self.StairSections`)))))
        (`/Game/SciFiModularEnvironment/SciFiRooms/HallwayStairSectionBP.HideStairs` _ashallway_stair_section_bp)
        (else
          (bind _returnvalue_3 (`AddComponent|NODE_AddChildActorComponent-0` :`bManualAttachment` true :`RelativeTransform` (`self.ActorTransform`)))
          (`ChildActorComponent.SetChildActorClass` _returnvalue_3 "/Game/SciFiModularEnvironment/SciFiRooms/HallwayStairSectionBP.HallwayStairSectionBP_C")
          (bind _ashallway_stair_section_bp_2 (cast `/Game/SciFiModularEnvironment/SciFiRooms/HallwayStairSectionBP` (`ChildActorComponent.ChildActor` _returnvalue_3)))
          (`KismetArrayLibrary.Array_AddUnique` (`self.StairSections`) _ashallway_stair_section_bp_2)
          (set `self.ActorTransform` (`SceneComponent.K2_GetComponentToWorld` (`/Game/SciFiModularEnvironment/SciFiRooms/HallwayStairSectionBP.Arrow` (`|GetArrayItem` (`self.StairSections`) _index)))))))))

(fn `UserConstructionScript`
  (`self.BuildStairs`)
  (`parent.UserConstructionScript`))