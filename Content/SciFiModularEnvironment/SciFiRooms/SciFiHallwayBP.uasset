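; SciFiHallwayBP is a modular sci-fi hallway that assembles itself in the construction script.
; With multiple sections, BuildHallway spawns additional HallwaySectionBP child actors, placing each at the previous piece's Arrow transform and recording it in HallwaySections.
; In that case it clears both end-door child actors.
; Otherwise, the DoorLeftEnd and DoorRightEnd flags decide whether each end gets a HallwayDoorBP.
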(fn `BuildHallway`
  (bind _doorleftendmesh (`self.DoorLeftEndMesh`))
  (bind _doorrightendmesh (`self.DoorRightEndMesh`))
  (set `self.ActorTransform` (`SceneComponent.K2_GetComponentToWorld` (`self.Arrow`)))
  (if (> (`self.NumberOfSections`) 1)
    (for _ (range (+ (- (`self.NumberOfSections`) 2) 1))
      (bind _returnvalue (`AddComponent|NODE_AddChildActorComponent-0` :`bManualAttachment` true :`RelativeTransform` (`self.ActorTransform`)))
      (`ChildActorComponent.SetChildActorClass` _returnvalue "/Game/SciFiModularEnvironment/SciFiRooms/HallwaySectionBP.HallwaySectionBP_C")
      (bind _ashallway_section_bp (cast `/Game/SciFiModularEnvironment/SciFiRooms/HallwaySectionBP` (`ChildActorComponent.ChildActor` _returnvalue) :!pure true))
      (set `self.ActorTransform` (`SceneComponent.K2_GetComponentToWorld` (`/Game/SciFiModularEnvironment/SciFiRooms/HallwaySectionBP.Arrow` _ashallway_section_bp)))
      (`ChildActorComponent.SetChildActorClass` (`self.DoorLeftEndMesh`) null)
      (`ChildActorComponent.SetChildActorClass` (`self.DoorRightEndMesh`) null)
      ;[1 0.8931 0.4316] Added
      (`KismetArrayLibrary.Array_AddUnique` (`self.HallwaySections`) _ashallway_section_bp))
    (else
      (`|ExecutionSequence`
        (:`then_0`
          (if (`self.DoorLeftEnd`)
            (`ChildActorComponent.SetChildActorClass` _doorleftendmesh "/Game/SciFiModularEnvironment/SciFiRooms/HallwayDoorBP.HallwayDoorBP_C")
            (else
              (`ChildActorComponent.SetChildActorClass` _doorleftendmesh null))))
        (:`then_1`
          (if (`self.DoorRightEnd`)
            (`ChildActorComponent.SetChildActorClass` _doorrightendmesh "/Game/SciFiModularEnvironment/SciFiRooms/HallwayDoorBP.HallwayDoorBP_C")
            (else
              (`ChildActorComponent.SetChildActorClass` _doorrightendmesh null))))))))

(fn `UserConstructionScript`
  (`self.BuildHallway`)
  (`parent.UserConstructionScript`))