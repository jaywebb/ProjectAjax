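; Modular medium sci-fi room piece that configures its six wall segments in the construction script.
; SetWallTypes reads per-wall Remove, Door or Window flags to clear each child actor or pick between two wall classes, then the parent construction script runs.
; Front segments reuse the back wall classes, only the left wall offers a window, and BackLeft/BackRight flags drive the opposite-named components.
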(fn `SetWallTypes`
  (bind _wallfrontleft (`self.WallFrontLeft`))
  (bind _wallfrontright (`self.WallFrontRight`))
  (bind _wallright (`self.WallRight`))
  (bind _wallleft (`self.WallLeft`))
  (bind _wallbackleft (`self.WallBackLeft`))
  (bind _wallbackright (`self.WallBackRight`))
  (`|ExecutionSequence`
    (:`then_0`
      (if (`self.RemoveBackRight`)
        (`ChildActorComponent.SetChildActorClass` (`self.WallBackLeft`) null)
        (elif (`self.DoorBackRight`)
          (`ChildActorComponent.SetChildActorClass` _wallbackleft "/Game/SciFiModularEnvironment/SciFiRooms/WallSMBack1.WallSMBack1_C")
          (else
            (`ChildActorComponent.SetChildActorClass` _wallbackleft "/Game/SciFiModularEnvironment/SciFiRooms/WallSMBack2.WallSMBack2_C")))))
    (:`then_1`
      (if (`self.RemoveBackLeft`)
        (`ChildActorComponent.SetChildActorClass` (`self.WallBackRight`) null)
        (elif (`self.DoorBackLeft`)
          (`ChildActorComponent.SetChildActorClass` _wallbackright "/Game/SciFiModularEnvironment/SciFiRooms/WallSMBack1.WallSMBack1_C")
          (else
            (`ChildActorComponent.SetChildActorClass` _wallbackright "/Game/SciFiModularEnvironment/SciFiRooms/WallSMBack2.WallSMBack2_C")))))
    (:`then_2`
      (if (`self.RemoveFrontLeft`)
        (`ChildActorComponent.SetChildActorClass` (`self.WallFrontLeft`) null)
        (elif (`self.DoorFrontLeft`)
          (`ChildActorComponent.SetChildActorClass` _wallfrontleft "/Game/SciFiModularEnvironment/SciFiRooms/WallSMBack1.WallSMBack1_C")
          (else
            (`ChildActorComponent.SetChildActorClass` _wallfrontleft "/Game/SciFiModularEnvironment/SciFiRooms/WallSMBack2.WallSMBack2_C")))))
    (:`then_3`
      (if (`self.RemoveFrontRight`)
        (`ChildActorComponent.SetChildActorClass` (`self.WallFrontRight`) null)
        (elif (`self.DoorFrontRight`)
          (`ChildActorComponent.SetChildActorClass` _wallfrontright "/Game/SciFiModularEnvironment/SciFiRooms/WallSMBack1.WallSMBack1_C")
          (else
            (`ChildActorComponent.SetChildActorClass` _wallfrontright "/Game/SciFiModularEnvironment/SciFiRooms/WallSMBack2.WallSMBack2_C")))))
    (:`then_4`
      (if (`self.RemoveRight`)
        (`ChildActorComponent.SetChildActorClass` (`self.WallRight`) null)
        (elif (`self.DoorRight`)
          (`ChildActorComponent.SetChildActorClass` _wallright "/Game/SciFiModularEnvironment/SciFiRooms/WallSMRight1.WallSMRight1_C")
          (else
            (`ChildActorComponent.SetChildActorClass` _wallright "/Game/SciFiModularEnvironment/SciFiRooms/WallSMRight2.WallSMRight2_C")))))
    (:`then_5`
      (if (`self.RemoveLeft`)
        (`ChildActorComponent.SetChildActorClass` (`self.WallLeft`) null)
        (elif (`self.WindowLeft`)
          (`ChildActorComponent.SetChildActorClass` _wallleft "/Game/SciFiModularEnvironment/SciFiRooms/WallSMLeft1.WallSMLeft1_C")
          (else
            (`ChildActorComponent.SetChildActorClass` _wallleft "/Game/SciFiModularEnvironment/SciFiRooms/WallSMLeft2.WallSMLeft2_C")))))))

(fn `UserConstructionScript`
  (`self.SetWallTypes`)
  (`parent.UserConstructionScript`))