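; RoomBaseBP is a base Blueprint for modular sci-fi rooms that applies one WallColor across a room's pieces.
; Its Construction Script walks all descendant components and calls SetWallColor on child actors that cast to WallBaseBP.
; Within that loop, it casts the root's owner (itself) to HallwayStairsBP or SciFiHallwayBP, recoloring their StairSections or HallwaySections on each wall found.
; The event graph is empty.
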(fn `UserConstructionScript`
  (bind _defaultsceneroot (`self.DefaultSceneRoot`))
  (bind _returnvalue (`ActorComponent.GetOwner` _defaultsceneroot))
  (for _array_element (`SceneComponent.GetChildrenComponents` _defaultsceneroot true)
    (bind _aswall_base_bp (cast `/Game/SciFiModularEnvironment/SciFiRooms/WallBaseBP` (`ChildActorComponent.ChildActor` (cast `ChildActorComponent` _array_element :!pure true))))
    (`/Game/SciFiModularEnvironment/SciFiRooms/WallBaseBP.SetWallColor` _aswall_base_bp (`self.Wall Color`))
    (bind _ashallway_stairs_bp (cast `/Game/SciFiModularEnvironment/SciFiRooms/HallwayStairsBP` _returnvalue)
      (:`then`
        (for _array_element_2 (`/Game/SciFiModularEnvironment/SciFiRooms/HallwayStairsBP.StairSections` _ashallway_stairs_bp)
          (`/Game/SciFiModularEnvironment/SciFiRooms/WallBaseBP.SetWallColor` _array_element_2 (`self.Wall Color`))))
      (:`CastFailed`
        (bind _assci_fi_hallway_bp (cast `/Game/SciFiModularEnvironment/SciFiRooms/SciFiHallwayBP` _returnvalue))
        (for _array_element_3 (`/Game/SciFiModularEnvironment/SciFiRooms/SciFiHallwayBP.HallwaySections` _assci_fi_hallway_bp)
          (`/Game/SciFiModularEnvironment/SciFiRooms/WallBaseBP.SetWallColor` _array_element_3 (`self.Wall Color`)))))))