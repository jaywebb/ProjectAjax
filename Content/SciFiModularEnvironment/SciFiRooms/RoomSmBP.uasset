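; RoomSmBP is a modular sci-fi room whose four walls are configured through per-side boolean options.
; The construction script runs SetWallType, then the parent's script, swapping each wall's child actor class or clearing it when that side is removed.
; Back, front and right choose door variants, while left chooses a window variant.
; Front reuses the back wall classes, and the event graph has no active logic.
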(fn `SetWallType`
  (bind _wall1 (`self.Wall1`))
  (bind _wall4 (`self.Wall4`))
  (bind _wall2 (`self.Wall2`))
  (bind _wall3 (`self.Wall3`))
  (`|ExecutionSequence`
    (:`then_0`
      (if (`self.RemoveBack`)
        (`ChildActorComponent.SetChildActorClass` (`self.Wall1`) null)
        (elif (`self.DoorBack`)
          (`ChildActorComponent.SetChildActorClass` _wall1 "/Game/SciFiModularEnvironment/SciFiRooms/WallSMBack1.WallSMBack1_C")
          (else
            (`ChildActorComponent.SetChildActorClass` _wall1 "/Game/SciFiModularEnvironment/SciFiRooms/WallSMBack2.WallSMBack2_C")))))
    (:`then_1`
      (if (`self.RemoveFront`)
        (`ChildActorComponent.SetChildActorClass` (`self.Wall4`) null)
        (elif (`self.DoorFront`)
          (`ChildActorComponent.SetChildActorClass` _wall4 "/Game/SciFiModularEnvironment/SciFiRooms/WallSMBack1.WallSMBack1_C")
          (else
            (`ChildActorComponent.SetChildActorClass` _wall4 "/Game/SciFiModularEnvironment/SciFiRooms/WallSMBack2.WallSMBack2_C")))))
    (:`then_2`
      (if (`self.RemoveRight`)
        (`ChildActorComponent.SetChildActorClass` (`self.Wall2`) null)
        (elif (`self.DoorRight`)
          (`ChildActorComponent.SetChildActorClass` _wall2 "/Game/SciFiModularEnvironment/SciFiRooms/WallSMRight1.WallSMRight1_C")
          (else
            (`ChildActorComponent.SetChildActorClass` _wall2 "/Game/SciFiModularEnvironment/SciFiRooms/WallSMRight2.WallSMRight2_C")))))
    (:`then_3`
      (if (`self.RemoveLeft`)
        (`ChildActorComponent.SetChildActorClass` (`self.Wall3`) null)
        (elif (`self.WindowLeft`)
          (`ChildActorComponent.SetChildActorClass` _wall3 "/Game/SciFiModularEnvironment/SciFiRooms/WallSMLeft1.WallSMLeft1_C")
          (else
            (`ChildActorComponent.SetChildActorClass` _wall3 "/Game/SciFiModularEnvironment/SciFiRooms/WallSMLeft2.WallSMLeft2_C")))))))

(fn `UserConstructionScript`
  (`self.SetWallType`)
  (`parent.UserConstructionScript`))