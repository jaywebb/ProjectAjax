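; HallwayConnectorBP is a modular sci-fi hallway junction that configures its four sides in the construction script.
; SetWallTypes sets each of the back, front, right and left child actor components to HallwayEndBP when its Remove flag is set, or to HallwaySectionBP otherwise.
; The parent construction script runs afterward, and the event graph holds only disabled stub events.
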(fn `SetWallTypes`
  (bind _hallwayleft (`self.HallwayLeft`))
  (bind _hallwayback (`self.HallwayBack`))
  (bind _hallwayfront (`self.HallwayFront`))
  (bind _hallwayright (`self.HallwayRight`))
  (`|ExecutionSequence`
    (:`then_0`
      (if (`self.RemoveBack`)
        (`ChildActorComponent.SetChildActorClass` _hallwayback "/Game/SciFiModularEnvironment/SciFiRooms/HallwayEndBP.HallwayEndBP_C")
        (else
          (`ChildActorComponent.SetChildActorClass` _hallwayback "/Game/SciFiModularEnvironment/SciFiRooms/HallwaySectionBP.HallwaySectionBP_C"))))
    (:`then_1`
      (if (`self.RemoveFront`)
        (`ChildActorComponent.SetChildActorClass` _hallwayfront "/Game/SciFiModularEnvironment/SciFiRooms/HallwayEndBP.HallwayEndBP_C")
        (else
          (`ChildActorComponent.SetChildActorClass` _hallwayfront "/Game/SciFiModularEnvironment/SciFiRooms/HallwaySectionBP.HallwaySectionBP_C"))))
    (:`then_2`
      (if (`self.RemoveRight`)
        (`ChildActorComponent.SetChildActorClass` _hallwayright "/Game/SciFiModularEnvironment/SciFiRooms/HallwayEndBP.HallwayEndBP_C")
        (else
          (`ChildActorComponent.SetChildActorClass` _hallwayright "/Game/SciFiModularEnvironment/SciFiRooms/HallwaySectionBP.HallwaySectionBP_C"))))
    (:`then_3`
      (if (`self.RemoveLeft`)
        (`ChildActorComponent.SetChildActorClass` _hallwayleft "/Game/SciFiModularEnvironment/SciFiRooms/HallwayEndBP.HallwayEndBP_C")
        (else
          (`ChildActorComponent.SetChildActorClass` _hallwayleft "/Game/SciFiModularEnvironment/SciFiRooms/HallwaySectionBP.HallwaySectionBP_C"))))))

(fn `UserConstructionScript`
  (`self.SetWallTypes`)
  (`parent.UserConstructionScript`))