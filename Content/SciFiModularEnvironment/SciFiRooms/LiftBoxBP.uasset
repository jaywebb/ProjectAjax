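; Moving cabin of a sci-fi lift that travels between two floors, working from state held in SciFiLiftBP.
; While Direction is non-zero, Tick locks the door and offsets the cabin vertically until it nears the destination.
; A resettable DoOnce then stops it, unlocks the door, swaps the destination floor and updates the UI widgets.
; A collision box sets SciFiLiftBP as the character's interact object and highlights the UI when stationary.
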(event `self.ReceiveBeginPlay`
  (bind _aslift_uiobject (cast `/Game/Blueprints/LIftUIObject` (`ChildActorComponent.ChildActor` (`self.LiftUIObject`))))
  (set `self.LiftUI` _aslift_uiobject)
  (bind _aslift_door_a (cast `/Game/SciFiModularEnvironment/SciFiRooms/LIftDoorA` (`ChildActorComponent.ChildActor` (`self.LiftDoor`))))
  (set `self.LIftDoorBP` _aslift_door_a))

(event `self.ReceiveTick`
  (params (DeltaSeconds :type "Float (single-precision)"))
  (bind _scifiliftbp (`self.SciFiLiftBP`))
  (bind _liftdoorbp (`self.LIftDoorBP`))
  (bind (_returnvalue_x _returnvalue_y _returnvalue_z) (`KismetMathLibrary.BreakVector` (`SceneComponent.K2_GetComponentLocation` (`self.Door`))))
  (bind (_destination_x _destination_y) (`KismetMathLibrary.BreakVector` (`/Game/SciFiModularEnvironment/SciFiRooms/SciFiLiftBP.Destination` (`self.SciFiLiftBP`))))
  ;[1 0.6226 0.1707] Only run if moving up or down
  (if (== (`self.Direction`) 0.0)
    _
    (elif (< (`KismetMathLibrary.VSize` (- (`/Game/SciFiModularEnvironment/SciFiRooms/SciFiLiftBP.Destination` _scifiliftbp) (`/Game/SciFiModularEnvironment/SciFiRooms/SciFiLiftBP.LiftCurrentLoc` _scifiliftbp))) (`/Game/SciFiModularEnvironment/SciFiRooms/SciFiLiftBP.AcceptableDistance` _scifiliftbp))
      (`self.ChangeFloor`)
      (else
        ;[1 0.821 0.4532] If you haven't reached the destination
        ;;[1 1 1] Hide the Interact Text
        (set `self.IsMoving` true)
        (set `/Game/SciFiModularEnvironment/SciFiRooms/LIftDoorA.IsLocked` true _liftdoorbp)
        (set `/Game/SciFiModularEnvironment/SciFiRooms/LIftDoorB.IsLocked` true (`/Game/SciFiModularEnvironment/SciFiRooms/LIftDoorA.LiftDoor` _liftdoorbp))
        ;;[1 1 1] Move Lift
        (`self.K2_AddActorLocalOffset` (`KismetMathLibrary.MakeVector` 0.0 0.0 (* (`self.Speed`) (* DeltaSeconds 10.0))))
        ;;[1 1 1] Update the lifts current location
        (set `/Game/SciFiModularEnvironment/SciFiRooms/SciFiLiftBP.LiftCurrentLoc` (`KismetMathLibrary.MakeVector` _destination_x _destination_y _returnvalue_z) (`self.SciFiLiftBP`))))))

(event `ChangeFloor`
  (bind _scifiliftbp (`self.SciFiLiftBP`))
  (bind _scifiliftbp_2 (`self.SciFiLiftBP`))
  (bind _scifiliftbp_3 (`self.SciFiLiftBP`))
  (bind _liftdoorbp (`self.LIftDoorBP`))
  (bind _liftui (`self.LiftUI`))
  (bind _liftwidget (`/Game/Blueprints/LIftUIObject.LiftWidget` _liftui))
  (bind _liftwidgetbgd (`/Game/Blueprints/LIftUIObject.LiftWidgetBgd` _liftui))
  (`/Engine/EditorBlueprintResources/StandardMacros.DoOnce` false :!label _label
    (:`Completed`
      ;[1 0.6861 0.3408] Stop the Lift and show the Interact Text
      (set `self.IsMoving` false)
      (set `self.Direction` 0.0)
      (set `/Game/SciFiModularEnvironment/SciFiRooms/LIftDoorA.IsLocked` false _liftdoorbp)
      (set `/Game/SciFiModularEnvironment/SciFiRooms/LIftDoorB.IsLocked` false (`/Game/SciFiModularEnvironment/SciFiRooms/LIftDoorA.LiftDoor` _liftdoorbp))
      ;[1 0.8987 0.3411] Determine the next destination and set the new destination. It is currently switching between only 2 destinations.
      (if (== (`/Game/SciFiModularEnvironment/SciFiRooms/SciFiLiftBP.CurrentFloor` _scifiliftbp_2) 1)
        (set `/Game/SciFiModularEnvironment/SciFiRooms/SciFiLiftBP.CurrentFloor` 2 _scifiliftbp_2)
        (set `/Game/SciFiModularEnvironment/SciFiRooms/SciFiLiftBP.Destination` (`SceneComponent.K2_GetComponentLocation` (`/Game/SciFiModularEnvironment/SciFiRooms/SciFiLiftBP.Floor2Marker` _scifiliftbp)) _scifiliftbp)
        (else
          (set `/Game/SciFiModularEnvironment/SciFiRooms/SciFiLiftBP.CurrentFloor` 1 _scifiliftbp_2)
          (set `/Game/SciFiModularEnvironment/SciFiRooms/SciFiLiftBP.Destination` (`SceneComponent.K2_GetComponentLocation` (`/Game/SciFiModularEnvironment/SciFiRooms/SciFiLiftBP.Floor1Marker` _scifiliftbp_3)) _scifiliftbp_3)))
      (`/Game/Blueprints/UI/LIftUI/LIftWidget.ShowFlashAnimation` _liftwidget true)
      (`/Game/Blueprints/UI/LIftUI/LIftWidgetBgd.ShowFlashAnimation` _liftwidgetbgd false)
      (`/Game/Blueprints/UI/LIftUI/LIftWidget.SetMoving` _liftwidget false)
      (if (`/Game/SciFiModularEnvironment/SciFiRooms/SciFiLiftBP.MovingUp` (`self.SciFiLiftBP`))
        (`/Game/Blueprints/UI/LIftUI/LIftWidgetBgd.SetDirection` _liftwidgetbgd false)
        (`/Game/Blueprints/UI/LIftUI/LIftWidget.SetDirection` _liftwidget false)
        (set `/Game/SciFiModularEnvironment/SciFiRooms/SciFiLiftBP.MovingUp` false (`self.SciFiLiftBP`))
        (else
          (`/Game/Blueprints/UI/LIftUI/LIftWidgetBgd.SetDirection` _liftwidgetbgd true)
          (`/Game/Blueprints/UI/LIftUI/LIftWidget.SetDirection` _liftwidget true)
          (set `/Game/SciFiModularEnvironment/SciFiRooms/SciFiLiftBP.MovingUp` true (`self.SciFiLiftBP`)))))))

(event `ResetFloorChange`
  (goto _label :!via `Reset`))

(event `self.CollisionBox.OnComponentBeginOverlap`
  (params (OverlappedComponent :type "PrimitiveComponent Object Reference") (OtherActor :type "Actor Object Reference") (OtherComp :type "PrimitiveComponent Object Reference") (OtherBodyIndex :type Integer) (bFromSweep :type Boolean) (SweepResult :type "HitResult Structure (by ref)"))
  ;[1 0.4962 0.2319] When entering the collision box in the lift, ( IF NOT MOVING ) set this lift as an Interact Object and show the Interact Text
  (bind _asals_anim_man_character_bp (cast `/Game/AdvancedLocomotionV4/Blueprints/CharacterLogic/ALS_AnimMan_CharacterBP` OtherActor))
  (set `/Game/AdvancedLocomotionV4/Blueprints/CharacterLogic/ALS_AnimMan_CharacterBP.InteractObject` (`self.SciFiLiftBP`) _asals_anim_man_character_bp)
  (if (not (`self.IsMoving`))
    (`/Game/Blueprints/UI/LIftUI/LIftWidget.SetActiveColor` (`/Game/Blueprints/LIftUIObject.LiftWidget` (`self.LiftUI`)) true)
    (`/Game/Blueprints/UI/LIftUI/LIftWidgetBgd.SetActiveColor` (`/Game/Blueprints/LIftUIObject.LiftWidgetBgd` (`self.LiftUI`)) true)))

(event `self.CollisionBox.OnComponentEndOverlap`
  (params (OverlappedComponent :type "PrimitiveComponent Object Reference") (OtherActor :type "Actor Object Reference") (OtherComp :type "PrimitiveComponent Object Reference") (OtherBodyIndex :type Integer))
  ;[1 0.8275 0.3664] When exiting the lift, set the Interact Object to NONE and hide the Interact Text
  (bind _asals_anim_man_character_bp (cast `/Game/AdvancedLocomotionV4/Blueprints/CharacterLogic/ALS_AnimMan_CharacterBP` OtherActor))
  (set `/Game/AdvancedLocomotionV4/Blueprints/CharacterLogic/ALS_AnimMan_CharacterBP.InteractObject` null _asals_anim_man_character_bp)
  (if (not (`self.IsMoving`))
    (`/Game/Blueprints/UI/LIftUI/LIftWidget.SetActiveColor` (`/Game/Blueprints/LIftUIObject.LiftWidget` (`self.LiftUI`)) false)
    (`/Game/Blueprints/UI/LIftUI/LIftWidgetBgd.SetActiveColor` (`/Game/Blueprints/LIftUIObject.LiftWidgetBgd` (`self.LiftUI`)) false)))

(fn `UserConstructionScript`)